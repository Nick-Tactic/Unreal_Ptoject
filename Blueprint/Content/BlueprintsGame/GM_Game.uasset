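; Game mode that runs the level flow: player spawning, death and respawn, and level completion.
; BeginPlay seeds the current checkpoint from the PlayerStart tagged "Start", where StartMatchFromUI spawns and possesses BP_Player.
; Deaths are counted on PS_Player, then a guarded delay leads to teleporting the same pawn to the checkpoint and restoring health, movement and input.
; CompleteLevel sets pause from its win flag and shows the win widget with UI-only input.
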(event `self.ReceiveBeginPlay`
  (bind _outactors (`GameplayStatics.GetAllActorsOfClass` "/Script/Engine.PlayerStart"))
  (for _array_element _outactors
    (if (== (`PlayerStart.PlayerStartTag` _array_element) "Start")
      (break)))
  (set `self.CurrentCheckpoint ` _array_element))

(event `StartMatchFromUI`
  (bind _returnvalue (`GameplayStatics.GetPlayerController` 0))
  (if (`self.HasMatchStarted`)
    (bind _returnvalue_2 (`|SpawnActorFromClass` "/Game/Blueprints/Character/BP_Player.BP_Player_C" (`self.GetTransform` (`self.CurrentCheckpoint `)) "AdjustIfPossibleButAlwaysSpawn" "MultiplyWithRoot" null null))
    (`Controller.Possess` _returnvalue _returnvalue_2)
    (set `self.PlayerPawn` _returnvalue_2)
    (`WidgetBlueprintLibrary.SetInputMode_GameOnly` _returnvalue)
    (set `PlayerController.bShowMouseCursor` false _returnvalue)))

(event `HandlePlayerDeath`
  (params (`DeadPawn ` :type "/Game/Blueprints/Character/BP_Player Object Reference"))
  (bind _bisrespawning (`self.bIsRespawning`))
  (if (not _bisrespawning)
    (bind _output_get (set `self.bIsRespawning` (not _bisrespawning)))
    (bind _asps_player (cast `/Game/Blueprints/Character/PS_Player` (`Pawn.PlayerState` `DeadPawn `)))
    (`/Game/Blueprints/Character/PS_Player.AddDeath` _asps_player)
    (`KismetSystemLibrary.Delay` 2.0)
    (`self.RespawnPlayer` `DeadPawn `)
    (set `self.bIsRespawning` (not _output_get))))

(event `CompleteLevel`
  (params (CanWin :type Boolean))
  (bind _returnvalue (`GameplayStatics.GetPlayerController` 0))
  (bind _output_get (set `self.bLevelComplete` CanWin))
  (`GameplayStatics.SetGamePaused` _output_get)
  (bind _returnvalue_2 (`|CreateWidget` "/Game/Widgets/WBP_Win.WBP_Win_C" _returnvalue))
  (`UserWidget.AddToViewport` _returnvalue_2 0)
  (`WidgetBlueprintLibrary.SetInputMode_UIOnlyEx` _returnvalue null))

(fn `RespawnPlayer`
  (params (`PawnToRevive ` :type "/Game/Blueprints/Character/BP_Player Object Reference"))
  (bind _currentcheckpoint_ (`self.CurrentCheckpoint `))
  (`/Engine/EditorBlueprintResources/StandardMacros.IsValid` `PawnToRevive `
    (:`Is Valid`
      (`/Engine/EditorBlueprintResources/StandardMacros.IsValid` _currentcheckpoint_
        (:`Is Valid`
          (`self.K2_SetActorLocationAndRotation` `PawnToRevive ` (`self.K2_GetActorLocation` _currentcheckpoint_) (`self.K2_GetActorRotation` _currentcheckpoint_) false true)
          (`/Game/Blueprints/Character/HealthComponent.ResetHealth` (`/Game/Blueprints/Character/BP_Player.Health` `PawnToRevive `))
          (`CharacterMovementComponent.SetMovementMode` (`Character.CharacterMovement` `PawnToRevive `) "MOVE_Walking" 0)
          (`self.EnableInput` `PawnToRevive ` (`GameplayStatics.GetPlayerController` 0))
          (return))))))

(fn `UserConstructionScript`)