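; Health component that tracks an actor's current health, with damage, heal and reset functions that raise health-changed and death events.
; Damage and healing are ignored at zero health, and both fire the change event before writing the clamped value.
; Lethal damage calls the death event without storing the new health.
; Non-lethal damage stores it and, for BP_Player owners, adds the amount to PS_Player's damage-taken total.
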(event `self.ReceiveBeginPlay`
  (set `self.CurrentHealth` (`self.MaxHealth`))
  (`self.OnHealthChanged`))

(fn `ApplyDamage`
  (params (`Amount ` :type "Float (double-precision)"))
  (bind _currenthealth (`self.CurrentHealth`))
  (bind _returnvalue (`KismetMathLibrary.FClamp` (- _currenthealth `Amount `) 0.0 (`self.MaxHealth`)))
  (if (not (<= _currenthealth 0.0))
    (`self.OnHealthChanged`)
    (if (<= _returnvalue 0.0)
      (`self.OnDeath`)
      (else
        (set `self.CurrentHealth` _returnvalue)
        (bind _asbp_player (cast `/Game/Blueprints/Character/BP_Player` (`self.GetOwner`)))
        (bind _asps_player (cast `/Game/Blueprints/Character/PS_Player` (`Pawn.PlayerState` _asbp_player)))
        (`/Game/Blueprints/Character/PS_Player.AddDamageTaken` _asps_player `Amount `))))
  (return))

(fn `Heal`
  (params (`Amount ` :type "Float (double-precision)"))
  (bind _currenthealth (`self.CurrentHealth`))
  (if (not (<= _currenthealth 0.0))
    (`self.OnHealthChanged`)
    (set `self.CurrentHealth` (`KismetMathLibrary.FClamp` (+ `Amount ` _currenthealth) 0.0 (`self.MaxHealth`))))
  (return))

(fn `ResetHealth`
  (set `self.CurrentHealth` (`self.MaxHealth`))
  (`self.OnHealthChanged`)
  (return))