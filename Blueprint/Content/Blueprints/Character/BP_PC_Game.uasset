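; Game player controller that puts up the start screen and a hold-to-view stats overlay.
; On BeginPlay it creates the WBP_Start widget, shows the mouse cursor and switches input to UI-only with focus on that widget.
; Pressing Tab creates and refreshes a WBP_Stats widget, and releasing Tab removes and clears it, with the StatsOpen flag guarding both.
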(event `self.ReceiveBeginPlay`
  (bind _aswbp_start (castclass `/Game/Widgets/WBP_Start` "/Game/Widgets/WBP_Start.WBP_Start_C"))
  (bind _returnvalue (`|CreateWidget` _aswbp_start self))
  (bind _output_get (set `self.StartWidget` _returnvalue))
  (`UserWidget.AddToViewport` _output_get 0)
  (set `self.bShowMouseCursor` true)
  (`WidgetBlueprintLibrary.SetInputMode_UIOnlyEx` self _output_get))

(event `Key|Tab`
  (params (Key :type "Key Structure"))
  (bind _bstatsopen (`self.bStatsOpen`))
  (bind _statswidget (`self.StatsWidget`))
  (bind _returnvalue (not _bstatsopen))
  (:`Pressed`
    (if (not _bstatsopen)
      (bind _returnvalue_2 (`|CreateWidget` "/Game/Widgets/WBP_Stats.WBP_Stats_C" self))
      (bind _output_get (set `self.StatsWidget` _returnvalue_2))
      (`UserWidget.AddToViewport` _output_get 0)
      (`/Game/Widgets/WBP_Stats.RefreshStats ` _output_get)
      (set `self.bStatsOpen` _returnvalue)))
  (:`Released`
    (if _bstatsopen
      (`/Engine/EditorBlueprintResources/StandardMacros.IsValid` _statswidget
        (:`Is Valid`
          (`Widget.RemoveFromParent` _statswidget)
          (set `self.StatsWidget` null))
        (:`Is Not Valid`
          _))
      (set `self.bStatsOpen` _returnvalue))))

(fn `UserConstructionScript`)