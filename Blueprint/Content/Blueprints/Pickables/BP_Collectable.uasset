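; BP_Collectable is an interactable pickup that counts as a collectable when the player interacts with it.
; OnInteract calls AddCollectable on GS_Game and AddPickup on the PS_Player at index 0, then destroys the actor.
; The Player input is unused, so the pickup always credits player state 0, and a failed cast stops the chain before the actor is destroyed.
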(fn `OnInteract`
  (params (Player :type "/Game/Blueprints/Character/BP_Player Object Reference"))
  (bind _asgs_game (cast `/Game/BlueprintsGame/GS_Game` (`GameplayStatics.GetGameState`)))
  (`/Game/BlueprintsGame/GS_Game.AddCollectable` _asgs_game)
  (bind _asps_player (cast `/Game/Blueprints/Character/PS_Player` (`GameplayStatics.GetPlayerState` 0)))
  (`/Game/Blueprints/Character/PS_Player.AddPickup` _asps_player)
  (`self.K2_DestroyActor`)
  (return))

(fn `UserConstructionScript`
  (`parent.UserConstructionScript`))