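; BP_ExitZone is the level exit, an interactable that completes the level when the win condition is met.
; On OnInteract it asks GS_Game whether the player can win and, if so, calls CompleteLevel on GM_Game.
; Otherwise it prints a Russian message saying there are not enough balls.
; All logic lives in OnInteract, as the overlap, tick and BeginPlay events are disabled.
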(fn `OnInteract`
  (params (Player :type "/Game/Blueprints/Character/BP_Player Object Reference"))
  (bind _asgs_game (cast `/Game/BlueprintsGame/GS_Game` (`GameplayStatics.GetGameState`)))
  (bind _canwin (`/Game/BlueprintsGame/GS_Game.CanWin` _asgs_game))
  (if _canwin
    (bind _asgm_game (cast `/Game/BlueprintsGame/GM_Game` (`GameplayStatics.GetGameMode`)))
    (`/Game/BlueprintsGame/GM_Game.CompleteLevel ` _asgm_game _canwin)
    (else
      (`KismetSystemLibrary.PrintString` "Шаров недостаточно!")))
  (return))

(fn `UserConstructionScript`
  (`parent.UserConstructionScript`))